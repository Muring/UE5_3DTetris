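; Game state Blueprint for a Tetris game that holds the score.
; The ScoreState event raises Score by one on each call.
; An unconnected branch would copy Score into HighestScore when the byte-converted score is larger, but it never runs, so the high score is not updated here.
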(event Custom|ScoreState
  (Variables|Default|SetScore (+ (Variables|Default|GetScore) 1)))

(event EventBeginPlay)

(event EventTick
  (params (DeltaSeconds :type Float%20%28single-precision%29)))

(fn ConstructionScript)